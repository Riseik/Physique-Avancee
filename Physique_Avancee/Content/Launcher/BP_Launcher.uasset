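; Slingshot-style launcher that lets the player drag to aim and fire a physics projectile, starting with TestMissile_BP.
; While shoot is held, Tick converts pointer drag into an impulse, predicts the trajectory and pulls the projectile opposite the launch direction.
; Release applies the impulse as a velocity change, then spawns a replacement after a delay, reusing BeginPlay's spawn path.
; Cancel stops aiming; power input and auto-zoom are empty stubs.
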(event Input|EnhancedActionEvents|EnhancedInputActionIA_CanceledShoot
  (params (ActionValue :type Boolean) (ElapsedSeconds :type Float%20%28double-precision%29) (TriggeredSeconds :type Float%20%28double-precision%29) (InputAction :type Input%20Action%20Object%20Reference :default "/Game/Input/Action/IA_CanceledShoot.IA_CanceledShoot"))
  (:Started
    (Variables|Default|SetShootPredict false)))

(event Input|EnhancedActionEvents|EnhancedInputActionIA_Shoot
  (params (ActionValue :type Boolean) (ElapsedSeconds :type Float%20%28double-precision%29) (TriggeredSeconds :type Float%20%28double-precision%29) (InputAction :type Input%20Action%20Object%20Reference :default "/Game/Input/Action/IA_Shoot.IA_Shoot"))
  (bind _ref_lanch_start (Variables|Default|GetRef%20Lanch%20Start))
  (bind _returnvalue (Transformation|GetWorldLocation _ref_lanch_start))
  (:Started
    (if (Variables|Default|GetCanShoot)
      (Variables|Default|SetShootPredict true)
      (bind _returnvalue_2 (Class|WidgetLayoutLibrary|GetMousePositiononPlatform))
      (Variables|Default|SetClick%20Original%20Pos _returnvalue_2)
      (if (Variables|Default|GetAuto%20Zoom)
        _)))
  (:Completed
    (if (Variables|Default|GetCanShoot)
      (if (Variables|Default|GetShootPredict)
        (Variables|Default|SetShootPredict false)
        (Physics|SetSimulatePhysics (Variables|Default|GetShapeComponent) true)
        (Physics|AddImpulse (Variables|Default|GetShapeComponent) (Math|Vector|MakeVector (Variables|Default|GetImpulse%20X) (Variables|Default|GetImpulse%20Y) (Variables|Default|GetImpulse%20Z)) "None" true)
        (Variables|Default|SetCanShoot false)
        (Transformation|SetWorldLocation (Variables|Default|GetLaunch%20Pos) _returnvalue false false)
        (Utilities|FlowControl|Delay 1.0)
        (bind _returnvalue_3 (Game|SpawnActorfromClass (Variables|Default|GetSelectedObject) (Math|Transform|MakeTransform _returnvalue "0, 0, 0" "1.000000,1.000000,1.000000") "Undefined" "MultiplyWithRoot" 0 0))
        (bind _output_get (Variables|Default|SetShapeComponent (Actor|GetComponentbyClass _returnvalue_3 "/Script/Engine.ShapeComponent")))
        (Physics|SetSimulatePhysics _output_get false)
        (Variables|Default|SetCanShoot true)))))

(event Input|EnhancedActionEvents|EnhancedInputActionIA_Power
  (params (ActionValue :type Float%20%28double-precision%29) (ElapsedSeconds :type Float%20%28double-precision%29) (TriggeredSeconds :type Float%20%28double-precision%29) (InputAction :type Input%20Action%20Object%20Reference :default "/Game/Input/Action/IA_Power.IA_Power")))

(event EventTick
  (params (DeltaSeconds :type Float%20%28single-precision%29))
  (bind _launch_pos (Variables|Default|GetLaunch%20Pos))
  (if (Variables|Default|GetShootPredict)
    (bind _returnvalue (Class|WidgetLayoutLibrary|GetMousePositiononPlatform))
    (Variables|Default|SetImpulse%20Z (* (.y (- _returnvalue (Variables|Default|GetClick%20Original%20Pos))) 5.0))
    (Variables|Default|SetImpulse%20X (* (* (.y (- _returnvalue (Variables|Default|GetClick%20Original%20Pos))) 5.0) 2.0))
    (Variables|Default|SetImpulse%20Y (* (.x (- _returnvalue (Variables|Default|GetClick%20Original%20Pos))) -5.0))
    (Class|GameplayStatics|BlueprintPredictProjectilePathbyTraceChannel (Transformation|GetWorldLocation _launch_pos) (Math|Vector|MakeVector (* (* (.y (- _returnvalue (Variables|Default|GetClick%20Original%20Pos))) 5.0) 2.0) (* (.x (- _returnvalue (Variables|Default|GetClick%20Original%20Pos))) -5.0) (* (.y (- _returnvalue (Variables|Default|GetClick%20Original%20Pos))) 5.0)) true 3e+01 "ECC_WorldDynamic" false 0 "ForDuration" 0.1 1e+01 1.0)
    (Transformation|SetWorldLocation (Variables|Default|GetShapeComponent) (+ (Transformation|GetWorldLocation (Variables|Default|GetRef%20Lanch%20Start)) (Math|Vector|MakeVector (* (Variables|Default|GetImpulse%20X) -0.05) (* (Variables|Default|GetImpulse%20Y) -0.1) (* (Variables|Default|GetImpulse%20Z) -0.1))) false false)
    (Transformation|SetWorldLocation _launch_pos (+ (Transformation|GetWorldLocation (Variables|Default|GetRef%20Lanch%20Start)) (Math|Vector|MakeVector (* (Variables|Default|GetImpulse%20X) -0.05) (* (Variables|Default|GetImpulse%20Y) -0.1) (* (Variables|Default|GetImpulse%20Z) -0.1))) false false)))

(event EventBeginPlay
  (Variables|Default|SetSelectedObject "/Game/TestMissile_BP.TestMissile_BP_C")
  (bind _returnvalue (Game|SpawnActorfromClass (Variables|Default|GetSelectedObject) (Math|Transform|MakeTransform (Transformation|GetWorldLocation (Variables|Default|GetRef%20Lanch%20Start)) "0, 0, 0" "1.000000,1.000000,1.000000") "Undefined" "MultiplyWithRoot" 0 0))
  (bind _output_get (Variables|Default|SetShapeComponent (Actor|GetComponentbyClass _returnvalue "/Script/Engine.ShapeComponent")))
  (Physics|SetSimulatePhysics _output_get false)
  (Variables|Default|SetCanShoot true))

(fn ConstructionScript)