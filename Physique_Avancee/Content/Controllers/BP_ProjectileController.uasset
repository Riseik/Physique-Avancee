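; Player controller for a launcher game that lets the player choose which projectile the BP_Launcher fires.
; BeginPlay finds the launcher, adds the input mapping, shows the cursor and fills a list of projectile classes.
; IA_Power scrolls through that list with wraparound and respawns the launcher's loaded actor.
; Other inputs cancel an aimed shot or trigger UseAbility on the parent-class projectiles found in the world.
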(event Custom|Action%20Mapping
  (Input|AddMappingContext (PlayerController|LocalPlayerSubsystems|GetEnhancedInputLocalPlayerSubsystem self) "/Game/Input/IMC_Default.IMC_Default" 0 "(bIgnoreAllPressedKeysUntilRelease=True,bForceImmediately=False,bNotifyUserSettings=False)"))

(event Custom|ScrollNegative
  (if (< (- (Variables|Default|GetIndexSelectedProjectile) 1) 0)
    (Variables|Default|SetIndexSelectedProjectile (- (Utilities|Array|Length (Variables|Default|GetProjectileList)) 1))
    (else
      (Variables|Default|SetIndexSelectedProjectile (- (Variables|Default|GetIndexSelectedProjectile) 1)))))

(event Custom|SetProjectileActor
  (bind _bp_launcher (Variables|Default|GetBP%20Launcher))
  (Default|DestroyCurrentActor (Variables|Default|GetBP%20Launcher))
  (Variables|/Game/Launcher/BP_Launcher.BP_Launcher_C|SetSelectedObject _bp_launcher (Utilities|Array|Get(acopy) (Variables|Default|GetProjectileList) (Variables|Default|GetIndexSelectedProjectile)))
  (Default|SpawnActor _bp_launcher))

(event Custom|ScrollPositive
  (if (>= (+ (Variables|Default|GetIndexSelectedProjectile) 1) (Utilities|Array|Length (Variables|Default|GetProjectileList)))
    (Variables|Default|SetIndexSelectedProjectile 0)
    (else
      (Variables|Default|SetIndexSelectedProjectile (+ (Variables|Default|GetIndexSelectedProjectile) 1)))))

(event Input|EnhancedActionEvents|EnhancedInputActionIA_CanceledShoot
  (params (ActionValue :type Boolean) (ElapsedSeconds :type Float%20%28double-precision%29) (TriggeredSeconds :type Float%20%28double-precision%29) (InputAction :type Input%20Action%20Object%20Reference :default "/Game/Input/Action/IA_CanceledShoot.IA_CanceledShoot"))
  (bind _bp_launcher (Variables|Default|GetBP%20Launcher))
  (:Started
    (Variables|/Game/Launcher/BP_Launcher.BP_Launcher_C|SetShootPredict _bp_launcher false)
    (Default|ResetLaunchPos _bp_launcher)
    (Default|ResetProjectilePos _bp_launcher)))

(event Input|EnhancedActionEvents|EnhancedInputActionIA_Power
  (params (ActionValue :type Float%20%28double-precision%29) (ElapsedSeconds :type Float%20%28double-precision%29) (TriggeredSeconds :type Float%20%28double-precision%29) (InputAction :type Input%20Action%20Object%20Reference :default "/Game/Input/Action/IA_Power.IA_Power"))
  (if (> ActionValue 0.0)
    (CallFunction|ScrollPositive)
    (else
      (CallFunction|ScrollNegative)))
  (CallFunction|SetProjectileActor))

(event EventBeginPlay
  (bind _projectilelist (Variables|Default|GetProjectileList))
  (bind _returnvalue (Actor|GetActorOfClass "/Game/Launcher/BP_Launcher.BP_Launcher_C"))
  (Variables|Default|SetBP%20Launcher _returnvalue)
  (CallFunction|ActionMapping)
  (Variables|Default|SetbShowMouseCursor true)
  (Utilities|Array|SetArrayElem _projectilelist 0 "/Game/Actors/Pawns/BP_BasicProjectile.BP_BasicProjectile_C")
  (Utilities|Array|SetArrayElem _projectilelist 1 "/Game/Actors/Pawns/BP_ExplosiveProjectile.BP_ExplosiveProjectile_C")
  (Utilities|Array|SetArrayElem _projectilelist 2 "/Game/Actors/Pawns/BP_TripleProjectile.BP_TripleProjectile_C")
  (Utilities|Array|SetArrayElem _projectilelist 3 "/Game/Actors/Pawns/BP_ParentProjectile.BP_ParentProjectile_C")
  (CallFunction|SetProjectileActor))

(event Input|ActionEvents|InputActionTriggerAbility
  (params (Key :type Key%20Structure :default "None"))
  (:Pressed
    (bind _outactors (Actor|GetAllActorsOfClass "/Game/Actors/Pawns/BP_ParentProjectile.BP_ParentProjectile_C"))
    (bind _output_get (Variables|Default|SetParentProjectile _outactors))
    (Default|UseAbility _output_get)))

(fn ConstructionScript)