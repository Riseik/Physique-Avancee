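; PC_BaseController is a player controller that sets up input and a starting test missile.
; On BeginPlay it adds the IMC_Default Enhanced Input mapping context and shows the mouse cursor.
; If BPLauncher and its LaunchPos are valid, it spawns TestMissile_BP there with physics simulation off.
; BP_Launcher actors are looked up, but the node assigning the first to BPLauncher is disconnected, so this graph never sets that reference.
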(event Custom|Action%20Mapping
  (Input|AddMappingContext (PlayerController|LocalPlayerSubsystems|GetEnhancedInputLocalPlayerSubsystem self) "/Game/Input/IMC_Default.IMC_Default" 0 "(bIgnoreAllPressedKeysUntilRelease=True,bForceImmediately=False,bNotifyUserSettings=False)"))

(event EventBeginPlay
  (bind _bp_launcher (Variables|Default|GetBP_Launcher))
  (bind _launch_pos (Variables|/Game/Launcher/BP_Launcher.BP_Launcher_C|GetLaunch%20Pos _bp_launcher))
  (bind _outactors (Actor|GetAllActorsOfClass "/Game/Launcher/BP_Launcher.BP_Launcher_C"))
  (CallFunction|ActionMapping)
  (Variables|/Script/Engine.PlayerController|SetbShowMouseCursor (Game|GetPlayerController 0) true)
  (Utilities|IsValid _bp_launcher
    (:Is%20Valid
      (Utilities|IsValid _launch_pos
        (:Is%20Valid
          (bind _returnvalue (Game|SpawnActorfromClass "/Game/TestMissile_BP.TestMissile_BP_C" (Math|Transform|MakeTransform (Transformation|GetWorldLocation _launch_pos) "0, 0, 0" "1.000000,1.000000,1.000000") "Undefined" "MultiplyWithRoot" 0 0))
          (bind _output_get (Variables|Default|SetTestMissileBP _returnvalue))
          (Physics|SetSimulatePhysics (Variables|/Game/TestMissile_BP.TestMissile_BP_C|GetTestMissilePhysics _output_get) false))))))

(fn ConstructionScript)