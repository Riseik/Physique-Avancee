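; BP_GrowingProjectile is a projectile Blueprint whose special ability makes it grow.
; It overrides the inherited UseAbility, calling the parent version and then setting the Sphere component's relative scale to a fixed, uniform larger size in a single step.
; The event graph and construction script add no logic of their own, so all other behavior comes from the parent class.
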(event EventBeginPlay
  (|CallParentFunction) ; Ce nœud est désactivé et ne sera pas appelé.\nFaites glisser les broches pour générer des fonctionnalités.
)

(event Collision|EventActorBeginOverlap
  (params (OtherActor :type Actor%20Object%20Reference))
  (|CallParentFunction OtherActor) ; Ce nœud est désactivé et ne sera pas appelé.\nFaites glisser les broches pour générer des fonctionnalités.
)

(event EventTick
  (params (DeltaSeconds :type Float%20%28single-precision%29))
  (|CallParentFunction DeltaSeconds) ; Ce nœud est désactivé et ne sera pas appelé.\nFaites glisser les broches pour générer des fonctionnalités.
)

(fn ConstructionScript
  (|CallParentFunction))

(fn UseAbility
  (|CallParentFunction)
  (Transformation|SetRelativeScale3D (Variables|Default|GetSphere) "3.000000,3.000000,3.000000"))